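; BP_Goal is a goal actor with a Score variable, a rep-notify and a text label showing the score.
; Tick runs a loop through a Delay into UpdateScore, so Score rises on a timer rather than from goals.
; OnRep_Score spawns an explosion emitter at the label and refreshes its text.
; The box overlap event is empty, and its soccer-ball overlap query is unused.
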(event `self.ReceiveBeginPlay`)

(event `self.ReceiveActorBeginOverlap`
  (params (OtherActor :type "Actor Object Reference")))

(event `self.ReceiveTick`
  (params (DeltaSeconds :type "Float (single-precision)"))
  (for _ (range 101)
    (`KismetSystemLibrary.Delay` 3.0)
    (`self.Update_Score`)))

(event `self.Box.OnComponentBeginOverlap`
  (params (OtherActor :type "Actor Object Reference") (OtherComp :type "PrimitiveComponent Object Reference") (OtherBodyIndex :type Integer) (bFromSweep :type Boolean) (SweepResult :type "EngineTypes.HitResult Structure (by ref)")))

(fn `OnRep_Score`
  (`GameplayStatics.SpawnEmitterAtLocation` "/Game/StarterContent/Particles/P_Explosion.P_Explosion" (`SceneComponent.K2_GetComponentLocation` (`self.ScoreLabel`)))
  (`TextRenderComponent.SetText` (`self.ScoreLabel`) (`KismetStringLibrary.Conv_IntToString` (`self.Score`))))

(fn `Update_Score`
  (set `self.Score` (+ (`self.Score`) 1)))

(fn `UserConstructionScript`)